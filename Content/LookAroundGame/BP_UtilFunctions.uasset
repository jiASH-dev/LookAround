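; BP_UtilFunctions holds a shared utility check for the LookAroundGame that filters overlap events by actor and component type.
; IsValidComponentAndActor first casts the overlapped actor to the requested class (character, platform or car).
; On success it casts the overlapped component to the requested kind (capsule, sphere, box, static or skeletal mesh), returning true only when both casts succeed.
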(fn IsValidComponentandActor
  (params (OverlappedActor :type Actor%20Object%20Reference) (OverlappedActorsComponent :type Actor%20Component%20Object%20Reference) (ComponentType :type E_ComponentType%20Enum :default "NewEnumerator0") (ActorType :type E_ActorType%20Enum :default "NewEnumerator0"))
  (Utilities|FlowControl|Sequence
    (:then_0
      (LocalVariables|SetOverlappedActorLocal OverlappedActor))
    (:then_1
      (LocalVariables|SetOverlappedActorsComponentLocal OverlappedActorsComponent))
    (:then_2
      (LocalVariables|SetComponentTypeLocal ComponentType))
    (:then_3
      (LocalVariables|SetActorTypeLocal ActorType))
    (:then_4
      (switch Utilities|FlowControl|Switch|SwitchonE_ActorType (LocalVariables|GetActorTypeLocal)
        (:NewEnumerator0
          (Utilities|Casting|CastToBP_Character (LocalVariables|GetOverlappedActorLocal)
            (:then
              _)
            (:CastFailed
              ;[1 1 1] Если это не переданный тип эктора пересекся
              (return false))))
        (:NewEnumerator1
          (Utilities|Casting|CastToBP_Platform (LocalVariables|GetOverlappedActorLocal)
            (:then
              _)
            (:CastFailed
              (return false))))
        (:NewEnumerator2
          (Utilities|Casting|CastToBP_Car (LocalVariables|GetOverlappedActorLocal)
            (:then
              _)
            (:CastFailed
              (return false)))))
      (switch Utilities|FlowControl|Switch|SwitchonE_ComponentType (LocalVariables|GetComponentTypeLocal)
        (:NewEnumerator0
          (Utilities|Casting|CastToCapsuleComponent (LocalVariables|GetOverlappedActorsComponentLocal)
            (:then
              ;[1 1 1] Если это персонаж и он пересекся капсулой, а не чем-то другим
              (return true))
            (:CastFailed
              ;[1 1 1] Если это переданный тип эктора, но он пересекся не капсулой
              (return false))))
        (:NewEnumerator1
          (Utilities|Casting|CastToSphereComponent (LocalVariables|GetOverlappedActorsComponentLocal)
            (:then
              ;[1 1 1] Если это переданнный тип эктора и он пересекся капсулой, а не чем-то другим
              (return true))
            (:CastFailed
              ;[1 1 1] Если это переданный тип эктора, но он пересекся не со сферой
              (return false))))
        (:NewEnumerator2
          (Utilities|Casting|CastToBoxComponent (LocalVariables|GetOverlappedActorsComponentLocal)
            (:then
              ;[1 1 1] Если это персонаж и он пересекся капсулой, а не чем-то другим
              (return true))
            (:CastFailed
              ;[1 1 1] Если это переданный тип эктора, но он пересекся не капсулой
              (return false))))
        (:NewEnumerator3
          (Utilities|Casting|CastToStaticMeshComponent (LocalVariables|GetOverlappedActorsComponentLocal)
            (:then
              ;[1 1 1] Если это персонаж и он пересекся капсулой, а не чем-то другим
              (return true))
            (:CastFailed
              ;[1 1 1] Если это переданный тип эктора, но он пересекся не капсулой
              (return false))))
        (:NewEnumerator4
          (Utilities|Casting|CastToSkeletalMeshComponent (LocalVariables|GetOverlappedActorsComponentLocal)
            (:then
              (return true))
            (:CastFailed
              (return false))))))))