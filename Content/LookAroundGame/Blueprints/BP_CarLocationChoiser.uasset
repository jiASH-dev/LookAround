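; BP_CarLocationChoiser picks a random spawn location for a car on a platform, using only Y lanes free of high barriers.
; A map seeded from the platform's environment component Y positions counts high barriers per lane through add and remove functions.
; GetIsAnyFreeYPosition also fills the free-lane list as a side effect.
; RandomizeCarPosition draws from that list, returns the matching world location on the last platform, then clears it.
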(event EventBeginPlay)

(event Collision|EventActorBeginOverlap
  (params (OtherActor :type Actor%20Object%20Reference)))

(event EventTick
  (params (DeltaSeconds :type Float%20%28single-precision%29)))

(fn ConstructionScript)

(fn AddHighBarrierYCoord
  (params (HeighBarrierYCoord :type Float%20%28single-precision%29))
  (bind _ypositionsbusycountermap (Variables|Default|GetYPositionsBusyCounterMap))
  (bind (_value _returnvalue) (Utilities|Map|Find _ypositionsbusycountermap HeighBarrierYCoord))
  (if _returnvalue
    ;[1 1 1] Если она там есть, мы берем ее значение и увеличиваем на 1
    (bind _result (Math|Integer|IncrementInt _value)
      (:%20%20
        (Utilities|Map|Add (Variables|Default|GetYPositionsBusyCounterMap) HeighBarrierYCoord _result)))
    (else
      ;[1 1 1] Если ее там не было, записываем новую Y позицию и присваиваем ей кол-во 1.
      (Utilities|Map|Add (Variables|Default|GetYPositionsBusyCounterMap) HeighBarrierYCoord 1))))

(fn RemoveHighBarrierYCoord
  (params (HighBarrierYCoord :type Float%20%28single-precision%29))
  (bind _ypositionsbusycountermap (Variables|Default|GetYPositionsBusyCounterMap))
  (bind (_value _returnvalue) (Utilities|Map|Find _ypositionsbusycountermap HighBarrierYCoord))
  (if _returnvalue
    (if (> _value 0)
      (bind _result (Math|Integer|DecrementInt _value)
        (:%20%20
          (Utilities|Map|Add (Variables|Default|GetYPositionsBusyCounterMap) HighBarrierYCoord _result))))))

(fn RandomizeCarPosition
  (params (LastPlatform :type BP%20Platform%20Object%20Reference))
  (bind _environmentscenecomponentworldlocation (Default|GetEnvironmenSceneComponentWorldLocationbyYPosition LastPlatform (Utilities|Array|Get(acopy) (Variables|Default|GetFreeYPositions) (Math|Random|RandomIntegerinRange 0 (Utilities|Array|LastIndex (Variables|Default|GetFreeYPositions))))))
  (Utilities|Array|Clear (Variables|Default|GetFreeYPositions))
  (return _environmentscenecomponentworldlocation))

(fn SetupYPositionsfromPlatform
  (params (Platform :type BP%20Platform%20Object%20Reference))
  (bind _environmentscenecomponents (Default|GetEnvironmentSceneComponents Platform))
  (for _array_element _environmentscenecomponents
    (Utilities|Map|Add (Variables|Default|GetYPositionsBusyCounterMap) (.Y (Math|Vector|BreakVector (Transformation|GetWorldLocation _array_element))) 0)))

(fn GetIsAnyFreeYPosition
  (bind _keys (Utilities|Map|Keys (Variables|Default|GetYPositionsBusyCounterMap)))
  (for _array_element _keys
    (if (.ReturnValue (Utilities|Map|Find (Variables|Default|GetYPositionsBusyCounterMap) _array_element))
      (if (== (.Value (Utilities|Map|Find (Variables|Default|GetYPositionsBusyCounterMap) _array_element)) 0)
        (Utilities|Array|Add (Variables|Default|GetFreeYPositions) _array_element))))
  (if (> (Utilities|Array|Length (Variables|Default|GetFreeYPositions)) 0)
    (return true)
    (else
      (return false))))