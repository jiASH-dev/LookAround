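; Spawn strategy actor that lays out a run of coins along a side shift pattern.
; SpawnCoinsBySide loops over a fixed range, spawning a BP_Coin at the current location and asking the supplied SideShiftStrategy for the next one.
; It returns the array of spawned coins; comments also mention a random count and a next-group position, neither of which the logic implements.
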(event EventBeginPlay)

(event Collision|EventActorBeginOverlap
  (params (OtherActor :type Actor%20Object%20Reference)))

(event EventTick
  (params (DeltaSeconds :type Float%20%28single-precision%29)))

(fn ConstructionScript)

(fn SpawnCoinsbySide
  (params (SideShiftStrategy :type BP%20Side%20Coins%20Shift%20Strategy%20Object%20Reference) (NewCoinSpawnLocation :type Vector))
  (LocalVariables|SetLastCoinSpawnLocationLocal NewCoinSpawnLocation)
  ;[1 1 1] Рандомим, сколько монет будет спавниться
  (for _index (range 0 5)
    ;[1 1 1] Спавним новую монету, меняем ссылку на последнюю монету и добавляем в массив
    (bind _returnvalue (Game|SpawnActorfromClass "/Game/LookAroundGame/Blueprints/Environment/BP_Coin.BP_Coin_C" (Math|Transform|MakeTransform (LocalVariables|GetLastCoinSpawnLocationLocal) "0, 0, 0" "1,1,1") "Undefined" 0 0))
    (bind _newcoinspawnlocation (Default|DoCoinsShift SideShiftStrategy (Transformation|GetActorLocation _returnvalue)))
    (LocalVariables|SetLastCoinSpawnLocationLocal _newcoinspawnlocation)
    (Utilities|Array|Add (LocalVariables|GetSpawnedCoinsLocal) _returnvalue))
  ;[1 1 1] После созданных монет создаем ответ для менеджера, в который заносим массив созданных монет и позицию, от которой можно спавнить следующую группу монет
  (return (LocalVariables|GetSpawnedCoinsLocal)))