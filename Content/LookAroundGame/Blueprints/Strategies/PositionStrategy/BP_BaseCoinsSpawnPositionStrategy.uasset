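; Base strategy actor for positioning coin spawns, with an empty SpawnCoins function that takes a spawn arrow.
; On BeginPlay it spawns Left, Forward and Right coin strategy actors and stores them in the BonusSpawnStrategies map under enum keys.
; RandomizeCoinsSpawnStrategies picks a random entry from a given CoinsShifts array and returns the matching strategy, while a getter exposes the whole map.
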(event EventBeginPlay
  (Utilities|FlowControl|Sequence
    (:then_0
      ;[1 1 1] Comment
      (bind _returnvalue (Game|SpawnActorfromClass "/Game/LookAroundGame/Blueprints/Strategies/SpawnStrategy/BP_LeftCoinsSpawnStrategy.BP_LeftCoinsSpawnStrategy_C" (Class|Util|GetDefaultActorTransform) "Undefined" 0 0))
      (Utilities|Map|Add (Variables|Default|GetBonusSpawnStrategies) "NewEnumerator1" _returnvalue))
    (:then_1
      ;[1 1 1] Comment
      (bind _returnvalue_2 (Game|SpawnActorfromClass "/Game/LookAroundGame/Blueprints/Strategies/SpawnStrategy/BP_ForwardCoinsSpawnStrategy.BP_ForwardCoinsSpawnStrategy_C" (Class|Util|GetDefaultActorTransform) "Undefined" 0 0))
      (Utilities|Map|Add (Variables|Default|GetBonusSpawnStrategies) "NewEnumerator2" _returnvalue_2))
    (:then_2
      ;[1 1 1] Comment
      (bind _returnvalue_3 (Game|SpawnActorfromClass "/Game/LookAroundGame/Blueprints/Strategies/SpawnStrategy/BP_RightCoinsSpawnStrategy.BP_RightCoinsSpawnStrategy_C" (Class|Util|GetDefaultActorTransform) "Undefined" 0 0))
      (Utilities|Map|Add (Variables|Default|GetBonusSpawnStrategies) "NewEnumerator0" _returnvalue_3))))

(fn ConstructionScript)

(fn SpawnCoins
  (params (BonusSpawnArrow :type Arrow%20Component%20Object%20Reference))
  (return 0))

(fn RandomizeCoinsSpawnStrategies
  (params (CoinsShifts :type Array%20of%20E_CoinsShift%20Enums :default "NewEnumerator0"))
  (return (.Value (Utilities|Map|Find (Variables|Default|GetBonusSpawnStrategies) (Utilities|Array|Get(acopy) CoinsShifts (Math|Random|RandomIntegerinRange 0 (Utilities|Array|LastIndex CoinsShifts)))))))

(fn GetBonusSpawnStrategies
  (return (Variables|Default|GetBonusSpawnStrategies)))