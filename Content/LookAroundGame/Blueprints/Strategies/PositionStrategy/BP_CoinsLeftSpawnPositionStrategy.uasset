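; BP_CoinsLeftSpawnPositionStrategy is a position strategy that decides where coins spawn, as the left-side variant.
; Its construction script configures a single bonus spawn position and a single coin shift from enum literals.
; SpawnCoins passes those shifts and positions, along with the given spawn arrow, to SpawnCoinsByShift and returns its result.
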(event EventBeginPlay
  (|CallParentFunction))

(fn ConstructionScript
  (Utilities|FlowControl|Sequence
    (:then_0
      (CallFunction|SetupSpawnPositions (Utilities|Array|MakeArray (Utilities|Enum|LiteralenumE_BonusSpawnPosition "NewEnumerator1"))))
    (:then_1
      (CallFunction|SetupBonusShifts (Utilities|Array|MakeArray (Utilities|Enum|LiteralenumE_CoinsShift "NewEnumerator1"))))))

(fn SpawnCoins
  (params (BonusSpawnArrow :type Arrow%20Component%20Object%20Reference))
  (bind _spawnedcoins (CallFunction|SpawnCoinsbyShift (CallFunction|GetBonusShifts) (CallFunction|GetSpawnPostitions) BonusSpawnArrow))
  (return _spawnedcoins))