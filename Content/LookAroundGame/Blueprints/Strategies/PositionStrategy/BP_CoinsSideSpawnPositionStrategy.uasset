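; Coin spawn-position strategy for the LookAround runner that places a forward coin stack with an optional side stack.
; On BeginPlay it spawns a forward-spawn strategy actor and caches the game mode.
; SpawnCoinsByShift collects shift strategies whose positions the game mode reports unoccupied, then spawns forward coins at the arrow.
; On a coin flip, a randomly chosen free shift continues a second stack from the last coin's location.
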(event EventBeginPlay
  (Utilities|FlowControl|Sequence
    (:then_0
      ;[1 1 1] Comment
      (|CallParentFunction))
    (:then_1
      ;[1 1 1] Comment
      (bind _returnvalue (Game|SpawnActorfromClass "/Game/LookAroundGame/Blueprints/Strategies/PositionStrategy/BP_CoinsForwardSpawnPositionStrategy.BP_CoinsForwardSpawnPositionStrategy_C" (Class|Util|GetDefaultActorTransform) "Undefined" 0 0))
      (Variables|Default|SetForwardFreeBonusSpawnStrategy _returnvalue))
    (:then_2
      ;[1 1 1] Comment
      (bind _asbp_look_around_game_mode (Utilities|Casting|CastToBP_LookAroundGameMode (Game|GetGameMode)))
      (Variables|Default|SetRunnerGameMode _asbp_look_around_game_mode))))

(fn ConstructionScript)

(fn SpawnCoinsbyShift
  (params (BonusShifts :type Array%20of%20E_CoinsShift%20Enums :default "NewEnumerator0") (PositionsToFindFree :type Array%20of%20E_BonusSpawnPosition%20Enums :default "NewEnumerator0") (BonusSpawnArrow :type Arrow%20Component%20Object%20Reference))
  (for (_array_element _array_index) PositionsToFindFree
    (bind _positionstatus (CallFunction|GetBonusSpawnPositionStatusbySpawnPosition _array_element))
    (if (not _positionstatus)
      (Utilities|Array|Add (LocalVariables|GetFreeBonusShifts) (Utilities|Array|Get(acopy) BonusShifts _array_index))))
  (bind _spawnedcoins (Default|SpawnCoins (Variables|Default|GetForwardFreeBonusSpawnStrategy) BonusSpawnArrow))
  (Utilities|Array|AppendArray (LocalVariables|GetAllSpawnedCoins) _spawnedcoins)
  ;[1 1 1] Рандомим, можем ли мы спавнить второй стак монет после первого
  (if (and (Math|Random|RandomBool) (> (Utilities|Array|Length (LocalVariables|GetFreeBonusShifts)) 0))
    (bind _spawnedcoins_2 (CallFunction|SpawnSecondCoinsStackbyStrategy (LocalVariables|GetFreeBonusShifts) (LocalVariables|GetAllSpawnedCoins)))
    (Utilities|Array|AppendArray (LocalVariables|GetAllSpawnedCoins) _spawnedcoins_2))
  (return (LocalVariables|GetAllSpawnedCoins)))

(fn SpawnSecondCoinsStackbyStrategy
  (params (FreeStrategies :type Array%20of%20E_CoinsShift%20Enums :default "NewEnumerator0") (AllSpawnedCoins :type Array%20of%20BP%20Coin%20Object%20References))
  (bind _randomizedbonusspawnstrategy (CallFunction|RandomizeCoinsSpawnStrategies FreeStrategies))
  (bind _spawnedcoins (Default|SpawnCoins _randomizedbonusspawnstrategy (Transformation|GetActorLocation (Utilities|Array|Get(acopy) AllSpawnedCoins (Utilities|Array|LastIndex AllSpawnedCoins)))))
  (return _spawnedcoins))

(fn GetBonusSpawnPositionStatusbySpawnPosition
  (params (SpawnPosition :type E_BonusSpawnPosition%20Enum :default "NewEnumerator0"))
  (bind _bonusspawnpositionstatuses (Default|GetBonusSpawnPositionStatuses (Variables|Default|GetRunnerGameMode)))
  (return (.Value (Utilities|Map|Find _bonusspawnpositionstatuses SpawnPosition))))

(fn SetupSpawnPositions
  (params (SpawnPositions :type Array%20of%20E_BonusSpawnPosition%20Enums :default "NewEnumerator0"))
  (Variables|Default|SetSpawnPositions SpawnPositions))

(fn SetupBonusShifts
  (params (BonusShifts :type Array%20of%20E_CoinsShift%20Enums :default "NewEnumerator0"))
  (Variables|Default|SetBonusShifts BonusShifts))

(fn GetSpawnPostitions
  (return (Variables|Default|GetSpawnPositions)))

(fn GetBonusShifts
  (return (Variables|Default|GetBonusShifts)))