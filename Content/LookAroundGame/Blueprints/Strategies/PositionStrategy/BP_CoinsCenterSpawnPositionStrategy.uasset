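; Coin spawn position strategy, named for center placement, that decides where bonus coins appear.
; Its construction script configures a fixed subset of spawn positions and coin shift options through inherited setup functions.
; SpawnCoins passes those shifts and positions, with the given spawn arrow, to SpawnCoinsByShift to find free spots and returns its result.
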(event EventBeginPlay
  (|CallParentFunction) ; This node is disabled and will not be called.\nDrag off pins to build functionality.
)

(event Collision|EventActorBeginOverlap
  (params (OtherActor :type Actor%20Object%20Reference)))

(event EventTick
  (params (DeltaSeconds :type Float%20%28single-precision%29)))

(fn ConstructionScript
  (Utilities|FlowControl|Sequence
    (:then_0
      (CallFunction|SetupSpawnPositions (Utilities|Array|MakeArray (Utilities|Enum|LiteralenumE_BonusSpawnPosition "NewEnumerator0") (Utilities|Enum|LiteralenumE_BonusSpawnPosition "NewEnumerator2"))))
    (:then_1
      (CallFunction|SetupBonusShifts (Utilities|Array|MakeArray (Utilities|Enum|LiteralenumE_CoinsShift "NewEnumerator0") (Utilities|Enum|LiteralenumE_CoinsShift "NewEnumerator1"))))))

(fn SpawnCoins
  (params (BonusSpawnArrow :type Arrow%20Component%20Object%20Reference))
  (bind _spawnedcoins (CallFunction|SpawnCoinsbyShift (CallFunction|GetBonusShifts) (CallFunction|GetSpawnPostitions) BonusSpawnArrow))
  (return _spawnedcoins))