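; Level manager for an endless runner that procedurally builds the track from chained platforms with obstacles, cars, coins and magnet pickups.
; BeginPlay spawns the factories, car location chooser and per-position coin strategies, then lays the starting track.
; Each LevelLimiter platform overlap appends a randomly populated platform at the last one's connection arrow.
; Spawned elements bind to InfluenceMediator, and bus positions feed the car location chooser as high barriers.
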(event Custom|CreateEnvironment
  ;[1 1 1] Таймер создается по причине того, что на момент запуска Play, Manager уже существует на уровне, его BeginPlay() отрабатывает быстрее, чем GameInstance или GameMode может оказаться в контексте уровня, поэтому крутим инициализацию до тех пор, пока не появится на уровне
  (CallFunction|SpawnPlatform)
  ;[1 1 1] Рандомим. Если выпало 0-40 и есть свободное место для спавна машины, то спавним машину, иначе- платформу без машины.
  (if (and (< (Math|Random|RandomIntegerinRange 0 100) 41) (Default|GetIsAnyFreeYPosition (Variables|Default|GetCarLocationChoiser)))
    (bind _spawncarlocation (Default|RandomizeCarPosition (Variables|Default|GetCarLocationChoiser) (Variables|Default|GetLastPlatform)))
    (bind _returnvalue (Game|SpawnActorfromClass "/Game/LookAroundGame/Blueprints/Environment/BP_Car.BP_Car_C" (Math|Transform|MakeTransform _spawncarlocation "0, 0, 0" "1,1,1") "Undefined" 0 0))
    (Default|BindtoInfluencedElement (Variables|Default|GetInfluenceMediator) _returnvalue))
  (bind _influencedelements (CallFunction|SpawnInfluenceElements))
  (for _array_element _influencedelements
    (Default|AddEnvironment (Variables|Default|GetLastPlatform) _array_element)
    (bind _asbp_bus (Utilities|Casting|CastToBP_Bus _array_element))
    (CallFunction|AddHighBarrierYCoordtoCarLocationChoiser _asbp_bus))
  (bind _bonusspawnpositionstatuses (Default|GetBonusSpawnPositionStatuses (Variables|Default|GetLastPlatform)))
  (Default|SetBonusSpawnPostitionStatuses (Variables|Default|GetRunnerGameMode) _bonusspawnpositionstatuses)
  (bind _spawnedcoins (CallFunction|SpawnCoins))
  (for _array_element_2 _spawnedcoins
    (Default|BindtoInfluencedElement (Variables|Default|GetInfluenceMediator) _array_element_2)
    (Default|AddEnvironment (Variables|Default|GetLastPlatform) _array_element_2))
  (if (< (Math|Random|RandomIntegerinRange 0 100) 31)
    (bind _bonus (CallFunction|SpawnBonus))
    (Default|BindtoInfluencedElement (Variables|Default|GetInfluenceMediator) _bonus)
    (Default|AddEnvironment (Variables|Default|GetLastPlatform) _bonus)))

(event EventBeginPlay
  (Utilities|FlowControl|Sequence
    (:then_0
      ;[1 1 1] Comment
      (bind _asbp_look_around_game_mode (Utilities|Casting|CastToBP_LookAroundGameMode (Game|GetGameMode)))
      (Variables|Default|SetRunnerGameMode _asbp_look_around_game_mode))
    (:then_1
      ;[1 1 1] Comment
      (bind _returnvalue (Game|SpawnActorfromClass "/Game/LookAroundGame/Blueprints/Strategies/PositionStrategy/BP_CoinsLeftSpawnPositionStrategy.BP_CoinsLeftSpawnPositionStrategy_C" (Math|Transform|MakeTransform "0, 0, 0") "Undefined" 0 0))
      (Utilities|Map|Add (Variables|Default|GetCoinsSpawnPositionsStrategies) "NewEnumerator0" _returnvalue)
      (bind _returnvalue_2 (Game|SpawnActorfromClass "/Game/LookAroundGame/Blueprints/Strategies/PositionStrategy/BP_CoinsRightSpawnPositionStrategy.BP_CoinsRightSpawnPositionStrategy_C" (Math|Transform|MakeTransform "0, 0, 0") "Undefined" 0 0))
      (Utilities|Map|Add (Variables|Default|GetCoinsSpawnPositionsStrategies) "NewEnumerator2" _returnvalue_2)
      (bind _returnvalue_3 (Game|SpawnActorfromClass "/Game/LookAroundGame/Blueprints/Strategies/PositionStrategy/BP_CoinsCenterSpawnPositionStrategy.BP_CoinsCenterSpawnPositionStrategy_C" (Math|Transform|MakeTransform "0, 0, 0") "Undefined" 0 0))
      (Utilities|Map|Add (Variables|Default|GetCoinsSpawnPositionsStrategies) "NewEnumerator1" _returnvalue_3)
      (bind _returnvalue_4 (Game|SpawnActorfromClass "/Game/LookAroundGame/Blueprints/Strategies/PositionStrategy/BP_CoinsForwardSpawnPositionStrategy.BP_CoinsForwardSpawnPositionStrategy_C" (Math|Transform|MakeTransform "0, 0, 0") "Undefined" 0 0))
      (Utilities|Map|Add (Variables|Default|GetCoinsSpawnPositionsStrategies) "NewEnumerator3" _returnvalue_4))
    (:then_2
      ;[1 1 1] Comment
      (bind _returnvalue_5 (Game|SpawnActorfromClass "/Game/LookAroundGame/Blueprints/BP_CarLocationChoiser.BP_CarLocationChoiser_C" (Class|Util|GetDefaultActorTransform) "Undefined" 0 0))
      (Variables|Default|SetCarLocationChoiser _returnvalue_5))
    (:then_3
      ;[1 1 1] Таймер создается по причине того, что на момент запуска Play, Manager уже существует на уровне, его BeginPlay() отрабатывает быстрее, чем GameInstance или GameMode может оказаться в контексте уровня, поэтому крутим инициализацию до тех пор, пока не появится на уровне
      (bind _outactors (Actor|GetAllActorsOfClass "/Game/LookAroundGame/Blueprints/BP_LevelLimiter.BP_LevelLimiter_C"))
      (Default|SetupCarLocationChoiser (Utilities|Array|Get(acopy) _outactors) (Variables|Default|GetCarLocationChoiser))
      (EventDispatchers|BindEventtoOnPlatformOverlapped (Utilities|Array|Get(acopy) _outactors) (delegate Custom|CreateEnvironment)))
    (:then_4
      ;[1 1 1] Comment
      (bind _returnvalue_6 (Game|SpawnActorfromClass "/Game/LookAroundGame/Blueprints/Factories/BP_InfluenceElementFactory.BP_InfluenceElementFactory_C" (Class|Util|GetDefaultActorTransform) "Undefined" 0 0))
      (Variables|Default|SetInfluenceElementFactory _returnvalue_6))
    (:then_5
      ;[1 1 1] Comment
      (bind _returnvalue_7 (Game|SpawnActorfromClass "/Game/LookAroundGame/Blueprints/Factories/BP_BonusElementFactory.BP_BonusElementFactory_C" (Class|Util|GetDefaultActorTransform) "Undefined" 0 0))
      (Variables|Default|SetBonusElementFactory _returnvalue_7))
    (:then_6
      ;[1 1 1] Comment
      (bind _outactors_2 (Actor|GetAllActorsOfClass "/Game/LookAroundGame/Blueprints/BP_InfluenceMediator.BP_InfluenceMediator_C"))
      (Variables|Default|SetInfluenceMediator (Utilities|Array|Get(acopy) _outactors_2)))
    (:then_7
      ;[1 1 1] Comment
      (CallFunction|SpawnBeginningEnvironment))))

(fn ConstructionScript)

(fn SpawnPlatform
  (Utilities|IsValid (Variables|Default|GetLastPlatform)
    (:Is%20Valid
      (bind _returnvalue (Game|SpawnActorfromClass "/Game/LookAroundGame/Blueprints/Environment/BP_Platform.BP_Platform_C" (Math|Transform|MakeTransform (Transformation|GetWorldLocation (Variables|/Game/LookAroundGame/Blueprints/Environment/BP_Platform.BP_Platform_C|GetConnectionArrowComponent (Variables|Default|GetLastPlatform))) "0, 0, 0" "1,1,1") "Undefined" 0 0))
      (bind _output_get (Variables|Default|SetLastPlatform _returnvalue))
      (return _output_get))
    (:Is%20Not%20Valid
      (bind _outactors (Actor|GetAllActorsOfClass "/Game/LookAroundGame/Blueprints/Character/BP_Character.BP_Character_C"))
      (bind _returnvalue_2 (Game|SpawnActorfromClass "/Game/LookAroundGame/Blueprints/Environment/BP_Platform.BP_Platform_C" (Math|Conversions|ToTransform(Vector) (Transformation|GetWorldLocation (Variables|/Script/Engine.Character|GetMesh (Utilities|Array|Get(acopy) _outactors)))) "Undefined" 0 0))
      (Variables|Default|SetLastPlatform _returnvalue_2)
      (return (Variables|Default|GetLastPlatform)))))

(fn SpawnInfluenceElements
  ;[1 1 1] Сколько будет спавниться препятствий
  (for _index (range 0 (Math|Random|RandomIntegerinRange 0 1))
    (bind _positionindex (CallFunction|RandomizePositionIndex))
    (bind _output_get (LocalVariables|SetSelectedIndexLocal _positionindex))
    (bind _environmentscenecomponent (Default|GetEnvironmentSceneComponentbyIndex (Variables|Default|GetLastPlatform) _output_get))
    (bind _influenceelement (Default|SpawnInfluenceElement (Variables|Default|GetInfluenceElementFactory) (Transformation|GetWorldLocation _environmentscenecomponent)))
    (Default|BindtoInfluencedElement (Variables|Default|GetInfluenceMediator) _influenceelement)
    (Utilities|Array|Add (LocalVariables|GetInfluencedElementsLocal) _influenceelement))
  (return (LocalVariables|GetInfluencedElementsLocal)))

(fn RandomizePositionIndex
  (bind _environmentscenecomponentslength (Default|GetEnvironmentSceneComponentsLength (Variables|Default|GetLastPlatform)))
  (return (Math|Random|RandomIntegerinRange 0 (- _environmentscenecomponentslength 1))))

(fn RandomizeBonusSpawn
  (params (BonusElementType :type E_BonusElementType%20Enum :default "NewEnumerator0"))
  (switch Utilities|FlowControl|Switch|SwitchonE_BonusElementType BonusElementType
    (:NewEnumerator0
      (if (> (Math|Random|RandomIntegerinRange 0 100) 90)
        _
        (else
          (return true))))
    (:NewEnumerator1
      (if (> (Math|Random|RandomIntegerinRange 0 100) 30)
        _
        (else
          (return true)))))
  (return false))

(fn SpawnBeginningEnvironment
  (for _index (range 0 15)
    (CallFunction|SpawnPlatform)
    (if (== _index 0)
      (Default|SetupYPositionsfromPlatform (Variables|Default|GetCarLocationChoiser) (Variables|Default|GetLastPlatform))
      (else
        (bind _influencedelements (CallFunction|SpawnInfluenceElements))
        (for _array_element _influencedelements
          (Default|AddEnvironment (Variables|Default|GetLastPlatform) _array_element)
          (bind _asbp_bus (Utilities|Casting|CastToBP_Bus _array_element))
          (CallFunction|AddHighBarrierYCoordtoCarLocationChoiser _asbp_bus))
        (bind _bonusspawnpositionstatuses (Default|GetBonusSpawnPositionStatuses (Variables|Default|GetLastPlatform)))
        (Default|SetBonusSpawnPostitionStatuses (Variables|Default|GetRunnerGameMode) _bonusspawnpositionstatuses)
        (bind _spawnedcoins (CallFunction|SpawnCoins))
        (for _array_element_2 _spawnedcoins
          (Default|BindtoInfluencedElement (Variables|Default|GetInfluenceMediator) _array_element_2)
          (Default|AddEnvironment (Variables|Default|GetLastPlatform) _array_element_2))
        (if (< (Math|Random|RandomIntegerinRange 0 100) 31)
          (bind _bonus (CallFunction|SpawnBonus))
          (Default|BindtoInfluencedElement (Variables|Default|GetInfluenceMediator) _bonus)
          (Default|AddEnvironment (Variables|Default|GetLastPlatform) _bonus))))))

(fn AddHighBarrierYCoordtoCarLocationChoiser
  (params (HighBarrier :type BP%20Bus%20Object%20Reference))
  (Default|AddHighBarrierYCoord (Variables|Default|GetCarLocationChoiser) (.Y (Math|Vector|BreakVector (Transformation|GetActorLocation HighBarrier)))))

(fn SpawnCoins
  (bind _bonusspawnruleswithoutroofs (Default|GetBonusSpawnRules (Variables|Default|GetLastPlatform)))
  (bind _bonusfreepositionindex (CallFunction|RandomizePlatformBonusFreePositionIndex _bonusspawnruleswithoutroofs))
  (LocalVariables|SetRandomizedBonusSpawnFreePosition (Utilities|Array|Get(acopy) _bonusspawnruleswithoutroofs _bonusfreepositionindex))
  (bind _spawnedcoins (Default|SpawnCoins (.Value (Utilities|Map|Find (Variables|Default|GetCoinsSpawnPositionsStrategies) (.BonusPosition (Utilities|Struct|BreakS_BonusSpawnRule (LocalVariables|GetRandomizedBonusSpawnFreePosition))))) (.BonusSpawnArrow (Utilities|Struct|BreakS_BonusSpawnRule (LocalVariables|GetRandomizedBonusSpawnFreePosition)))))
  (return _spawnedcoins))

(fn SpawnBonus
  (bind _bonusspawnruleswithoutroofs (Default|GetBonusSpawnRules (Variables|Default|GetLastPlatform)))
  (bind _bonusfreepositionindex (CallFunction|RandomizePlatformBonusFreePositionIndex _bonusspawnruleswithoutroofs))
  (bind _returnvalue (Game|SpawnActorfromClass "/Game/LookAroundGame/Blueprints/Environment/BP_Magnet.BP_Magnet_C" (Math|Conversions|ToTransform(Vector) (Transformation|GetWorldLocation (.BonusSpawnArrow (Utilities|Struct|BreakS_BonusSpawnRule (Utilities|Array|Get(acopy) _bonusspawnruleswithoutroofs _bonusfreepositionindex))))) "Undefined" 0 0))
  (return _returnvalue))

(fn RandomizePlatformBonusFreePositionIndex
  (params (PlatformBonusFreePositions :type Array%20of%20S%20Bonus%20Spawn%20Rule%20Structures))
  (return (Math|Random|RandomIntegerinRange 0 (Utilities|Array|LastIndex PlatformBonusFreePositions))))