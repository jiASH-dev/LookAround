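; Moving car hazard for the runner game that triggers its influence event when it hits the character.
; MoveEnvironment shifts it along -X at five times the game mode's max speed, keeping its last speed when the world stops on player death.
; BeginPlay starts a looping MoveEnvironment timer targeting the game mode, not the car.
; A front box lowers obstacles on overlap and raises them afterwards; the wheel-spin function is never run.
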(event OnComponentBeginOverlap(FrontBoxCollisionComponent)
  (params (OverlappedComponent :type Primitive%20Component%20Object%20Reference) (OtherActor :type Actor%20Object%20Reference) (OtherComp :type Primitive%20Component%20Object%20Reference) (OtherBodyIndex :type Integer) (bFromSweep :type Boolean) (SweepResult :type Hit%20Result%20Structure%20%28by%20ref%29))
  (bind _asbp_obstacle (Utilities|Casting|CastToBP_Obstacle OtherActor))
  (Default|StartDown _asbp_obstacle))

(event OnComponentHit(BoxCollisionComponent)
  (params (HitComponent :type Primitive%20Component%20Object%20Reference) (OtherActor :type Actor%20Object%20Reference) (OtherComp :type Primitive%20Component%20Object%20Reference) (NormalImpulse :type Vector :default "0, 0, 0") (Hit :type Hit%20Result%20Structure%20%28by%20ref%29))
  (Utilities|Casting|CastToBP_Character OtherActor)
  (Default|CallOnInfluence))

(event OnComponentEndOverlap(FrontBoxCollisionComponent)
  (params (OverlappedComponent :type Primitive%20Component%20Object%20Reference) (OtherActor :type Actor%20Object%20Reference) (OtherComp :type Primitive%20Component%20Object%20Reference) (OtherBodyIndex :type Integer))
  (bind _asbp_obstacle (Utilities|Casting|CastToBP_Obstacle OtherActor))
  (Default|StartUp _asbp_obstacle))

(event EventBeginPlay
  (|CallParentFunction)
  (bind _asbp_look_around_game_mode (Utilities|Casting|CastToBP_LookAroundGameMode (Game|GetGameMode)))
  (bind _output_get (Variables|Default|SetRunnerGameMode _asbp_look_around_game_mode))
  (Utilities|Time|SetTimerbyFunctionName _output_get "MoveEnvironment" 0.01 true))

(fn ConstructionScript)

(fn SpinWheels
  (for _array_element (Components|GetChildrenComponents (Variables|Default|GetEnvironmentMeshComponent) false)
    (Transformation|SetRelativeRotation _array_element (Math|Rotator|MakeRotator (+ (.Roll (Math|Rotator|BreakRotator (Variables|/Script/Engine.SceneComponent|GetRelativeRotation _array_element))) 2.2e+02) 0.0 (.Yaw (Math|Rotator|BreakRotator (Variables|/Script/Engine.SceneComponent|GetRelativeRotation _array_element)))) false false)))

(fn MoveEnvironment
  (bind _returnvalue (Transformation|GetActorLocation))
  (bind _returnvalue_2 (Transformation|GetActorLocation))
  (bind (_x _y _z) (Math|Vector|BreakVector _returnvalue))
  (bind (_x_2 _y_2 _z_2) (Math|Vector|BreakVector _returnvalue_2))
  (bind _maxspeed (Default|GetMaxSpeed (Variables|Default|GetRunnerGameMode)))
  ;[1 1 1] Когда игрок погибает, весь энвайронмент останавливается, но машина должна продолжать ехать.
  (if (== _maxspeed 0.0)
    (Transformation|SetActorLocation (Math|Vector|MakeVector (- _x_2 (Variables|Default|GetLastCorrectXSpeed)) _y_2 _z_2) false false)
    (else
      (bind _output_get (Variables|Default|SetLastCorrectXSpeed (* 5 _maxspeed)))
      (Transformation|SetActorLocation (Math|Vector|MakeVector (- _x _output_get) _y _z) false false))))

(fn DestroyActor
  (Utilities|Time|ClearTimerbyFunctionName 0 "MoveEnvironment")
  (Actor|DestroyActor))