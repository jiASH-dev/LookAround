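; BP_Platform is a three-lane level segment that tracks where environment objects and bonuses can spawn and destroys its environment objects along with itself.
; Construction builds left, center and right slots and bonus rules, and slot getters remove each slot they hand out.
; AddEnvironment matches non-BP_Obstacle objects to lanes by world Y, removing that bonus rule and marking it occupied.
; A BP_Bus also contributes its own arrow as a fourth bonus position.
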(event EventBeginPlay
  (|CallParentFunction))

(event EventTick
  (params (DeltaSeconds :type Float%20%28single-precision%29))
  (|CallParentFunction DeltaSeconds))

(fn ConstructionScript
  (Variables|Default|SetBonusSpawnRules (Utilities|Array|MakeArray (Utilities|Struct|MakeS_BonusSpawnRule (Variables|Default|GetLeftBonusSpawnArrowComponent) "NewEnumerator0") (Utilities|Struct|MakeS_BonusSpawnRule (Variables|Default|GetCenterBonusSpawnArrowComponent) "NewEnumerator1") (Utilities|Struct|MakeS_BonusSpawnRule (Variables|Default|GetRightBonusSpawnArrowComponent) "NewEnumerator2")))
  (Variables|Default|SetEnvironmentSceneComponents (Utilities|Array|MakeArray (Variables|Default|GetEnvironmentLeftPositionSceneComponent) (Variables|Default|GetEnvironmentCenterPositionSceneComponent) (Variables|Default|GetEnvironmentRightPositionSceneComponent)))
  (Utilities|Map|Add (Variables|Default|GetBonusSpawnPositionsStatuses) "NewEnumerator0" false)
  (Utilities|Map|Add (Variables|Default|GetBonusSpawnPositionsStatuses) "NewEnumerator1" false)
  (Utilities|Map|Add (Variables|Default|GetBonusSpawnPositionsStatuses) "NewEnumerator2" false))

(fn GetEnvironmentSceneComponentbyIndex
  (params (EnvironmentSceneComponentIndex :type Integer))
  (LocalVariables|SetEnvironmentSceneComponentLocal (Utilities|Array|Get(acopy) (Variables|Default|GetEnvironmentSceneComponents) EnvironmentSceneComponentIndex))
  (Utilities|Array|RemoveIndex (Variables|Default|GetEnvironmentSceneComponents) EnvironmentSceneComponentIndex)
  (return (LocalVariables|GetEnvironmentSceneComponentLocal)))

(fn GetEnvironmentSceneComponentsLength
  (return (Utilities|Array|Length (Variables|Default|GetEnvironmentSceneComponents))))

(fn AddEnvironment
  (params (Environment :type BP%20Environment%20Object%20Reference))
  ;[1 1 1] Проверяет, если заспавнили большое препятствие, то удаляет стрелку для спавна бонуса напротив большого препяствия, потому как оно загораживает место спавна
  (Utilities|Casting|CastToBP_Obstacle Environment
    (:then
      _)
    (:CastFailed
      (CallFunction|RemoveBonusSpawnRule Environment)))
  (Utilities|Array|Add (Variables|Default|GetEnvironments) Environment)
  (bind _asbp_bus (Utilities|Casting|CastToBP_Bus Environment))
  (Utilities|Array|Add (Variables|Default|GetBonusSpawnRules) (Utilities|Struct|MakeS_BonusSpawnRule (Variables|/Game/LookAroundGame/Blueprints/Environment/BP_Bus.BP_Bus_C|GetBonusSpawnArrowComponent _asbp_bus) "NewEnumerator3")))

(fn GetEnvironmenSceneComponentWorldLocationbyYPosition
  (params (YPosition :type Float%20%28single-precision%29))
  (for _array_element (Variables|Default|GetEnvironmentSceneComponents)
    (bind _output_get (LocalVariables|SetEnvironmentSceneComponentWorldLocationLocal (Transformation|GetWorldLocation _array_element)))
    (if (== (.Y (Math|Vector|BreakVector _output_get)) YPosition)
      (Utilities|Array|RemoveItem (Variables|Default|GetEnvironmentSceneComponents) _array_element)
      (return (LocalVariables|GetEnvironmentSceneComponentWorldLocationLocal)))))

(fn Destroy
  (for _array_element (Variables|Default|GetEnvironments)
    (Utilities|IsValid _array_element
      (:Is%20Valid
        (Actor|DestroyActor _array_element))))
  (Actor|DestroyActor))

(fn GetEnvironments
  (return (Variables|Default|GetEnvironments)))

(fn RemoveBonusSpawnRule
  (params (Environment :type BP%20Environment%20Object%20Reference))
  (for (_array_element _array_index) (Variables|Default|GetBonusSpawnRules)
    (if (== (.Y (Math|Vector|BreakVector (Transformation|GetActorLocation Environment))) (.Y (Math|Vector|BreakVector (Transformation|GetWorldLocation (.BonusSpawnArrow (Utilities|Struct|BreakS_BonusSpawnRule _array_element))))))
      ;[1 1 1] Вносим занятую позицию в массив для того, чтобы знать, какие позиции занятые для спавна бонусов
      (CallFunction|ChangeBonusSpawnPositionStatus (.BonusPosition (Utilities|Struct|BreakS_BonusSpawnRule (Utilities|Array|Get(acopy) (Variables|Default|GetBonusSpawnRules) _array_index))))
      (Utilities|Array|RemoveIndex (Variables|Default|GetBonusSpawnRules) _array_index))))

(fn ChangeBonusSpawnPositionStatus
  (params (OccupiedBonusSpawnPosition :type E_BonusSpawnPosition%20Enum :default "NewEnumerator0"))
  (Utilities|Map|Add (Variables|Default|GetBonusSpawnPositionsStatuses) OccupiedBonusSpawnPosition true))

(fn GetBonusSpawnPositionStatuses
  (return (Variables|Default|GetBonusSpawnPositionsStatuses)))

(fn GetEnvironmentSceneComponentsYPositions
  (return (Utilities|Array|MakeArray (.Y (Math|Vector|BreakVector (Transformation|GetWorldLocation (Variables|Default|GetEnvironmentLeftPositionSceneComponent)))) (.Y (Math|Vector|BreakVector (Transformation|GetWorldLocation (Variables|Default|GetEnvironmentCenterPositionSceneComponent)))) (.Y (Math|Vector|BreakVector (Transformation|GetWorldLocation (Variables|Default|GetEnvironmentRightPositionSceneComponent)))))))

(fn GetEnvironmentSceneComponents
  (return (Variables|Default|GetEnvironmentSceneComponents)))

(fn GetBonusSpawnRules
  (return (Variables|Default|GetBonusSpawnRules)))