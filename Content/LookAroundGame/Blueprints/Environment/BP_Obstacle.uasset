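; BP_Obstacle is an environment barrier that sinks and rises vertically, and signals an influence event when a valid actor and component overlap its collision box.
; StartDown and StartUp each clear both movement timers, then start a fast looping timer that steps the actor's Z by a shift amount.
; Lowering stops when the arrow component reaches the root height cached at construction, and raising stops when the root returns to it.
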(event OnComponentBeginOverlap(BoxCollisionComponent)
  (params (OverlappedComponent :type Primitive%20Component%20Object%20Reference) (OtherActor :type Actor%20Object%20Reference) (OtherComp :type Primitive%20Component%20Object%20Reference) (OtherBodyIndex :type Integer) (bFromSweep :type Boolean) (SweepResult :type Hit%20Result%20Structure%20%28by%20ref%29))
  (bind _overlappedresult (CallFunction|IsValidComponentandActor OtherActor OtherComp "NewEnumerator0" "NewEnumerator0"))
  (if _overlappedresult
    (Default|CallOnInfluence)))

(event EventBeginPlay
  (|CallParentFunction))

(event EventTick
  (params (DeltaSeconds :type Float%20%28single-precision%29))
  (|CallParentFunction DeltaSeconds))

(fn ConstructionScript
  (Variables|Default|SetStartRootZPosition (.Z (Math|Vector|BreakVector (Transformation|GetWorldLocation (Variables|Default|GetDefaultSceneRoot))))))

(fn GetDown
  (bind _returnvalue (Transformation|GetActorLocation))
  (bind (_x _y _z) (Math|Vector|BreakVector _returnvalue))
  (if (<= (.Z (Math|Vector|BreakVector (Transformation|GetWorldLocation (Variables|Default|GetShiftingArrowComponent)))) (Variables|Default|GetStartRootZPosition))
    (Utilities|Time|ClearTimerbyFunctionName 0 "GetDown")
    (else
      (Transformation|SetActorLocation (Math|Vector|MakeVector _x _y (- _z (Class|Util|GetBarrierUpandDownShift))) false false))))

(fn GetUp
  (bind _returnvalue (Transformation|GetActorLocation))
  (bind (_x _y _z) (Math|Vector|BreakVector _returnvalue))
  (if (>= (.Z (Math|Vector|BreakVector (Transformation|GetWorldLocation (Variables|Default|GetDefaultSceneRoot)))) (Variables|Default|GetStartRootZPosition))
    (Utilities|Time|ClearTimerbyFunctionName 0 "GetUp")
    (else
      (Transformation|SetActorLocation (Math|Vector|MakeVector _x _y (+ _z (Class|Util|GetBarrierUpandDownShift))) false false))))

(fn StartDown
  (Utilities|Time|ClearTimerbyFunctionName 0 "GetDown")
  (Utilities|Time|ClearTimerbyFunctionName 0 "GetUp")
  (Utilities|Time|SetTimerbyFunctionName 0 "GetDown" 0.01 true))

(fn StartUp
  (Utilities|Time|ClearTimerbyFunctionName 0 "GetDown")
  (Utilities|Time|ClearTimerbyFunctionName 0 "GetUp")
  (Utilities|Time|SetTimerbyFunctionName 0 "GetUp" 0.01 true))