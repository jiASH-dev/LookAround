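; BP_InfluenceElementFactory is a factory Blueprint that spawns random obstacle actors, called influence elements, at a given position.
; SpawnInfluenceElement picks a random E_ObstacleType from the enum's entry count, then switches on it to spawn and return a fence, bus or stone platform.
; All logic lives in that one function; the event graph and construction script are empty.
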(event EventBeginPlay)

(event Collision|EventActorBeginOverlap
  (params (OtherActor :type Actor%20Object%20Reference)))

(event EventTick
  (params (DeltaSeconds :type Float%20%28single-precision%29)))

(fn ConstructionScript)

(fn SpawnInfluenceElement
  (params (Position :type Vector))
  (switch Utilities|FlowControl|Switch|SwitchonE_ObstacleType (Utilities|Enum|ByteToEnumE_ObstacleType (Math|Conversions|ToByte(Integer) (Math|Random|RandomIntegerinRange 0 (- (|GetNumEnumEntries) 1))))
    (:NewEnumerator0
      (bind _returnvalue (Game|SpawnActorfromClass "/Game/LookAroundGame/Blueprints/Environment/BP_Fence.BP_Fence_C" (Math|Transform|MakeTransform Position "0, 0, 0" "1,1,1") "Undefined" 0 0))
      (return _returnvalue))
    (:NewEnumerator3
      (bind _returnvalue_2 (Game|SpawnActorfromClass "/Game/LookAroundGame/Blueprints/Environment/BP_Bus.BP_Bus_C" (Math|Transform|MakeTransform Position "0, 0, 0" "1,1,1") "Undefined" 0 0))
      (return _returnvalue_2))
    (:NewEnumerator4
      (bind _returnvalue_3 (Game|SpawnActorfromClass "/Game/LookAroundGame/Blueprints/Environment/BP_StonePlatform.BP_StonePlatform_C" (Math|Transform|MakeTransform Position "0, 0, 0" "1,1,1") "Undefined" 0 0))
      (return _returnvalue_3))))