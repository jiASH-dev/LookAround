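; Meteor spawner that periodically drops a BP_Meteor near the player character on a random Y position taken from BP_Platform.
; A looping timer places a danger-zone decal below the character, then a one-shot timer replaces it with a meteor spawned at a point offset above and along negative X.
; Short polling timers resolve the character and Y positions, while BP_InfluenceMediator binds each meteor and can stop the spawn loop.
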(event Custom|DoStopMeteorAndDangerZone
  (CallFunction|StopMeteorandDangerZone))

(event EventBeginPlay
  (CallFunction|InitInfluenceMediator)
  (EventDispatchers|BindEventtoOnStopMeteorandDangerZone (Variables|Default|GetInfluenceMediator) (delegate Custom|DoStopMeteorAndDangerZone))
  (Utilities|Time|SetTimerbyFunctionName 0 "InitCharacter" 0.001 true)
  (Utilities|Time|SetTimerbyFunctionName 0 "InitYPositions" 0.001 true)
  (Utilities|Time|SetTimerbyFunctionName 0 "StartMeteorAndDangerZone" 4.0 true))

(fn ConstructionScript)

(fn StartMeteorandDangerZone
  (bind _returnvalue (Math|Vector|MakeVector -0.5 0.0 0.5))
  (bind _character (Variables|Default|GetCharacter))
  (bind _ypositions (Variables|Default|GetYPositions))
  (bind _character_2 (Variables|Default|GetCharacter))
  (bind _returnvalue_2 (Transformation|GetActorLocation _character_2))
  (bind _returnvalue_3 (* _returnvalue 4e+02))
  (bind _returnvalue_4 (+ _returnvalue_2 _returnvalue_3))
  (bind (_x _y _z) (Math|Vector|BreakVector _returnvalue_4))
  (if (and (!= (Utilities|Array|Length (Variables|Default|GetYPositions)) 0) (Utilities|IsValid (Variables|Default|GetCharacter)))
    (LocalVariables|SetCurrentYSpawnPosition (Utilities|Array|Get(acopy) _ypositions (Math|Random|RandomIntegerinRange 0 (Utilities|Array|LastIndex _ypositions))))
    (bind _skeletalmeshcomponent (Default|GetMesh _character))
    (CallFunction|StartDangerZone (Math|Vector|MakeVector (.X (Math|Vector|BreakVector (Transformation|GetActorLocation _character))) (LocalVariables|GetCurrentYSpawnPosition) (- (.Z (Math|Vector|BreakVector (Transformation|GetWorldLocation _skeletalmeshcomponent))) 1e+02)))
    (Variables|Default|SetCurrentMeteorSpawnPosition (Math|Vector|MakeVector _x (LocalVariables|GetCurrentYSpawnPosition) _z))
    (Utilities|Time|SetTimerbyFunctionName 0 "StopDangerZoneAndStartMeteor" 1.0)))

(fn StartDangerZone
  (params (SpawnPosition :type Vector))
  (bind _returnvalue (Game|SpawnActorfromClass "/Script/Engine.DecalActor" (Math|Transform|MakeTransform SpawnPosition "0, 0, 0" "1,1,1") "Undefined" 0 0))
  (bind _output_get (Variables|Default|SetCurrentDangerZoneDecal _returnvalue))
  (Rendering|Components|Decal|SetDecalMaterial (Variables|/Script/Engine.DecalActor|GetDecal _output_get) "/Game/LookAroundGame/Materials/M_DangerZone.M_DangerZone"))

(fn StartMeteor
  (bind _returnvalue (Game|SpawnActorfromClass "/Game/LookAroundGame/Blueprints/Environment/BP_Meteor.BP_Meteor_C" (Math|Transform|MakeTransform (Variables|Default|GetCurrentMeteorSpawnPosition) "0, 0, 0" "1,1,1") "Undefined" 0 0))
  (Default|BindtoMeteor (Variables|Default|GetInfluenceMediator) _returnvalue))

(fn InitCharacter
  (Utilities|IsValid (Variables|Default|GetCharacter)
    (:Is%20Valid
      (Utilities|Time|ClearTimerbyFunctionName 0 "InitCharacter"))
    (:Is%20Not%20Valid
      (bind _outactors (Actor|GetAllActorsOfClass "/Game/LookAroundGame/Blueprints/Character/BP_Character.BP_Character_C"))
      (Variables|Default|SetCharacter (Utilities|Array|Get(acopy) _outactors)))))

(fn FindLocationUnderCharacter
  (bind _character (Variables|Default|GetCharacter))
  (bind _returnvalue (Transformation|GetActorLocation _character))
  (bind _outhit (Collision|LineTraceByChannel _returnvalue (- _returnvalue "0,0.000000,600.000000") "TraceTypeQuery1" false (Utilities|Array|MakeArray _character) "None"))
  (return (.Location (Collision|BreakHitResult _outhit))))

(fn InitInfluenceMediator
  (bind _outactors (Actor|GetAllActorsOfClass "/Game/LookAroundGame/Blueprints/BP_InfluenceMediator.BP_InfluenceMediator_C"))
  (Variables|Default|SetInfluenceMediator (Utilities|Array|Get(acopy) _outactors)))

(fn StopMeteorandDangerZone
  (Utilities|Time|ClearTimerbyFunctionName 0 "StartMeteorAndDangerZone"))

(fn StopDangerZoneandStartMeteor
  (Actor|DestroyActor (Variables|Default|GetCurrentDangerZoneDecal))
  (CallFunction|StartMeteor))

(fn SetYPositions
  (params (YPositions :type Array%20of%20Floats%20%28single-precision%29))
  (Variables|Default|SetYPositions YPositions))

(fn InitYPositions
  (if (== (Utilities|Array|Length (Variables|Default|GetYPositions)) 0)
    (bind _outactors (Actor|GetAllActorsOfClass "/Game/LookAroundGame/Blueprints/Environment/BP_Platform.BP_Platform_C"))
    (bind _environmentscenecomponentsypositions (Default|GetEnvironmentSceneComponentsYPositions (Utilities|Array|Get(acopy) _outactors)))
    (Variables|Default|SetYPositions _environmentscenecomponentsypositions)
    (else
      (Utilities|Time|ClearTimerbyFunctionName 0 "InitYPositions"))))