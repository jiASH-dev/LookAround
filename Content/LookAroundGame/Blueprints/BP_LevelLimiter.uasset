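; BP_LevelLimiter is a trigger box in the runner game that destroys platforms and cars that overlap it.
; For platforms, it first removes the Y coordinates of their bus high barriers from the car location chooser.
; Each removed platform also fires the platform-overlapped call and feeds a counter that periodically raises the game mode's max speed while it is below a cap.
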(event OnComponentBeginOverlap(BoxComponent)
  (params (OverlappedComponent :type Primitive%20Component%20Object%20Reference) (OtherActor :type Actor%20Object%20Reference) (OtherComp :type Primitive%20Component%20Object%20Reference) (OtherBodyIndex :type Integer) (bFromSweep :type Boolean) (SweepResult :type Hit%20Result%20Structure%20%28by%20ref%29))
  (bind _overlappedresult (CallFunction|IsValidComponentandActor OtherActor OtherComp "NewEnumerator2" "NewEnumerator1"))
  (if _overlappedresult
    (bind _asbp_platform (Utilities|Casting|CastToBP_Platform OtherActor))
    (bind _environments (Default|GetEnvironments _asbp_platform))
    (for _array_element _environments
      (bind _asbp_bus (Utilities|Casting|CastToBP_Bus _array_element))
      (CallFunction|RemoveHightBarrierfromPlatform _asbp_bus))
    (Default|Destroy _asbp_platform)
    (CallFunction|SetMaxSpeedifAvaliable)
    (Default|CallOnPlatformOverlapped)
    (else
      (bind _overlappedresult_2 (CallFunction|IsValidComponentandActor OtherActor OtherComp "NewEnumerator3" "NewEnumerator2"))
      (if _overlappedresult_2
        (bind _asbp_car (Utilities|Casting|CastToBP_Car OtherActor))
        (Default|DestroyActor _asbp_car)))))

(event EventBeginPlay
  (bind _asbp_look_around_game_mode (Utilities|Casting|CastToBP_LookAroundGameMode (Game|GetGameMode)))
  (Variables|Default|SetRunnerGameMode _asbp_look_around_game_mode))

(fn ConstructionScript)

(fn SetMaxSpeedifAvaliable
  (bind _maxspeed (Default|GetMaxSpeed (Variables|Default|GetRunnerGameMode)))
  (if (< _maxspeed 15.0)
    (Math|Integer|IncrementInt (Variables|Default|GetOverlappedPlatformsCounter)
      (:%20%20
        (if (== (Math|Integer|%(Integer) (Variables|Default|GetOverlappedPlatformsCounter) 15) 0)
          (bind _maxspeed_2 (Default|GetMaxSpeed (Variables|Default|GetRunnerGameMode)))
          (Default|SetMaxSpeed (Variables|Default|GetRunnerGameMode) (+ _maxspeed_2 2.0)))))))

(fn SetupCarLocationChoiser
  (params (CarLocationChoiser :type BP%20Car%20Location%20Choiser%20Object%20Reference))
  (Variables|Default|SetCarLocationChoiser CarLocationChoiser))

(fn RemoveHightBarrierfromPlatform
  (params (HighBarrier :type BP%20Bus%20Object%20Reference))
  (Default|RemoveHighBarrierYCoord (Variables|Default|GetCarLocationChoiser) (.Y (Math|Vector|BreakVector (Transformation|GetActorLocation HighBarrier)))))