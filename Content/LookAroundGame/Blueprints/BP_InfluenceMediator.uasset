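; Mediator for the runner game that turns obstacle, bus, car, meteor, magnet and coin events into player effects.
; BeginPlay creates the HUD, caches the game mode and polls by timer for the character.
; Bind events cast each element and subscribe its handler.
; Lethal hits stop the world, kill the character and broadcast a meteor/danger-zone stop; magnets grant a timed pickup area with hand mesh, coins add points.
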(event Custom|BindToInfluencedElement
  (params (InfluencedElement :type BP%20Influence%20Element%20Object%20Reference))
  ;[1 1 1] Можно будет переделать под мапу
  (Variables|Default|SetCurrentInfluenceElement InfluencedElement)
  (Utilities|FlowControl|Sequence
    (:then_0
      (bind _asbp_obstacle (Utilities|Casting|CastToBP_Obstacle (Variables|Default|GetCurrentInfluenceElement)))
      (EventDispatchers|BindEventtoOnInfluence _asbp_obstacle (delegate Custom|KillCharacterByObstacleAndStopTheWorld)))
    (:then_1
      (bind _asbp_bus (Utilities|Casting|CastToBP_Bus (Variables|Default|GetCurrentInfluenceElement)))
      (EventDispatchers|BindEventtoOnInfluence _asbp_bus (delegate Custom|KillCharacterByBusAndStopTheWorld)))
    (:then_2
      (bind _asbp_magnet (Utilities|Casting|CastToBP_Magnet (Variables|Default|GetCurrentInfluenceElement)))
      (EventDispatchers|BindEventtoOnInfluence _asbp_magnet (delegate Custom|AddCharacterMagnetPower)))
    (:then_3
      (bind _asbp_coin (Utilities|Casting|CastToBP_Coin (Variables|Default|GetCurrentInfluenceElement)))
      (EventDispatchers|BindEventtoOnInfluence _asbp_coin (delegate Custom|GivePointsAndDraw)))
    (:then_4
      (bind _asbp_car (Utilities|Casting|CastToBP_Car (Variables|Default|GetCurrentInfluenceElement)))
      (EventDispatchers|BindEventtoOnInfluence _asbp_car (delegate Custom|KillCharacterByDynamicAndStopTheWorld)))))

(event Custom|AddCharacterMagnetPower
  ;[1 1 1] Можно будет переделать под мапу
  (Transformation|SetWorldScale3D (Variables|/Game/LookAroundGame/Blueprints/Character/BP_Character.BP_Character_C|GetMagnetArea (Variables|Default|GetCharacter)) "20.000000,20.000000,20.000000")
  ;;[1 1 1] Если у персонажа уже есть в руке что-то, то не добавляем снова.
  (Utilities|IsValid (Variables|Default|GetCurrentBuffStaticMeshActor)
    (:Is%20Valid
      _)
    (:Is%20Not%20Valid
      (bind _buffstaticmeshactor (CallFunction|CreateBuffStaticMeshActor))
      (Transformation|AttachComponentToComponent _buffstaticmeshactor (Variables|/Script/Engine.Character|GetMesh (Variables|Default|GetCharacter)) (Class|SkinnedMeshComponent|GetSocketBoneName (Variables|/Script/Engine.Character|GetMesh (Variables|Default|GetCharacter)) "Buff") "KeepRelative" "KeepRelative" "KeepRelative" true)))
  (Utilities|Time|SetTimerbyEvent (delegate Custom|StopMagnetArea) 7.0))

(event Custom|GivePointsAndDraw
  ;[1 1 1] Можно будет переделать под мапу
  (Rendering|Components|TextRender|SetText (Variables|/Game/LookAroundGame/UI/WBP_HUD.WBP_HUD_C|GetPointsText (Variables|Default|GetHUD)) (Utilities|Text|ToText(Integer) (+ 5 (Math|Conversions|ToInteger(Byte) (Utilities|String|ToString(Text) (Class|TextBlock|GetText (Variables|/Game/LookAroundGame/UI/WBP_HUD.WBP_HUD_C|GetPointsText (Variables|Default|GetHUD))))))))
  (Default|SetPoints (Variables|Default|GetCharacter) 1))

(event Custom|StopMagnetArea
  ;[1 1 1] Можно будет переделать под мапу
  (Transformation|SetWorldScale3D (Variables|/Game/LookAroundGame/Blueprints/Character/BP_Character.BP_Character_C|GetMagnetArea (Variables|Default|GetCharacter)) "0, 0, 0")
  (Actor|DestroyActor (Variables|Default|GetCurrentBuffStaticMeshActor)))

(event Custom|KillCharacterByBusAndStopTheWorld
  ;[1 1 1] Можно будет переделать под мапу
  (Default|StopMove (Variables|Default|GetCharacter))
  (Default|SetMaxSpeed (Variables|Default|GetRunnerGameMode) 0.0)
  (if (Default|GetIsCharacterCurrentPositionMoreThanNew (Variables|Default|GetCharacter))
    (if (Default|GetIsCharacterLanded (Variables|Default|GetCharacter))
      (Default|KillCharacterWithoutPhysics (Variables|Default|GetCharacter) "NewEnumerator1")
      (else
        (Default|KillCharacterWithoutPhysics (Variables|Default|GetCharacter) "NewEnumerator3")))
    (elif (Default|GetIsCharacterLanded (Variables|Default|GetCharacter))
      (Default|KillCharacterWithoutPhysics (Variables|Default|GetCharacter) "NewEnumerator2")
      (else
        (Default|KillCharacterWithoutPhysics (Variables|Default|GetCharacter) "NewEnumerator4"))))
  (Default|CallOnStopMeteorandDangerZone))

(event Custom|KillCharacterByObstacleAndStopTheWorld
  ;[1 1 1] Можно будет переделать под мапу
  (Default|SetMaxSpeed (Variables|Default|GetRunnerGameMode) 0.0)
  (Default|KillCharacterWithoutPhysics (Variables|Default|GetCharacter) "NewEnumerator0")
  (Default|CallOnStopMeteorandDangerZone))

(event Custom|BindToMeteor
  (params (Meteor :type BP%20Meteor%20Object%20Reference))
  ;[1 1 1] Можно будет переделать под мапу
  (EventDispatchers|BindEventtoOnStoptheWorldandKillCharacter Meteor (delegate Custom|KillCharacterByDynamicAndStopTheWorld)))

(event Custom|KillCharacterByDynamicAndStopTheWorld
  ;[1 1 1] Можно будет переделать под мапу
  (Default|SetMaxSpeed (Variables|Default|GetRunnerGameMode) 0.0)
  (Default|KillCharacterwithPhysics (Variables|Default|GetCharacter))
  (Default|CallOnStopMeteorandDangerZone))

(event EventBeginPlay
  (Utilities|FlowControl|Sequence
    (:then_0
      (CallFunction|CreateHUDandAddtoScreen))
    (:then_1
      (Utilities|Time|SetTimerbyFunctionName 0 "CharacterInit" 0.01 true))
    (:then_2
      (bind _asbp_look_around_game_mode (Utilities|Casting|CastToBP_LookAroundGameMode (Game|GetGameMode)))
      (Variables|Default|SetRunnerGameMode _asbp_look_around_game_mode))))

(fn ConstructionScript)

(fn CreateHUDandAddtoScreen
  (bind _returnvalue (UserInterface|CreateWidget "/Game/LookAroundGame/UI/WBP_HUD.WBP_HUD_C"))
  (bind _output_get (Variables|Default|SetHUD _returnvalue))
  (UserInterface|Viewport|AddtoPlayerScreen _output_get))

(fn CreateBuffStaticMeshActor
  (bind _returnvalue (Game|SpawnActorfromClass "/Script/Engine.StaticMeshActor" (Transformation|GetSocketTransform (Variables|/Script/Engine.Character|GetMesh (Variables|Default|GetCharacter)) "Buff" "RTS_ParentBoneSpace") "Undefined" 0 0))
  (bind _output_get (Variables|Default|SetCurrentBuffStaticMeshActor _returnvalue))
  (Transformation|SetMobility _output_get "Movable")
  (Components|StaticMesh|SetStaticMesh (Variables|/Script/Engine.StaticMeshActor|GetStaticMeshComponent (Variables|Default|GetCurrentBuffStaticMeshActor)) "/Game/LookAroundGame/Meshes/SM_Magnet.SM_Magnet")
  (return (Variables|Default|GetCurrentBuffStaticMeshActor)))

(fn CharacterInit
  (bind _outactors (Actor|GetAllActorsOfClass "/Game/LookAroundGame/Blueprints/Character/BP_Character.BP_Character_C"))
  (Utilities|IsValid (Utilities|Array|Get(acopy) _outactors)
    (:Is%20Valid
      (Variables|Default|SetCharacter (Utilities|Array|Get(acopy) _outactors))
      (Utilities|Time|ClearTimerbyFunctionName 0 "CharacterInit"))))