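; BP_Character is the runner's player character, handling lane moves, jumps, rolls, dashes and death.
; DoMove tweens Y on the Moving timeline, while Tick pins X to an accumulator that super jump advances until landing, carrying the attached level limiter.
; StartDashDown rolls on the ground, tracing for fences to drop capsule collision, or pulls down airborne via a looping timer.
; State flags are exposed through getters, and death either ragdolls or stores a hit animation.
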(event OnComponentHit(CapsuleComponent)
  (params (HitComponent :type Primitive%20Component%20Object%20Reference) (OtherActor :type Actor%20Object%20Reference) (OtherComp :type Primitive%20Component%20Object%20Reference) (NormalImpulse :type Vector :default "0, 0, 0") (Hit :type Hit%20Result%20Structure%20%28by%20ref%29))
  ;[1 1 1] Comment
  (Utilities|Casting|CastToBP_Environment OtherActor)
  (Variables|Default|SetIsCharacterLanded true)
  (Variables|/Script/Engine.CharacterMovementComponent|SetJumpZVelocity (Variables|Character|GetCharacterMovement) 6e+02)
  (Variables|Default|SetXShiftValue 0.0))

(event Custom|DoMove
  (params (NewYPosition :type Float%20%28single-precision%29))
  (bind _returnvalue (Transformation|GetActorLocation))
  (bind (_x _y _z) (Math|Vector|BreakVector _returnvalue))
  ;[1 1 1] Comment
  (bind _output_get (Variables|Default|SetNewYPosition NewYPosition))
  (Audio|Components|Audio|Stop (Variables|Default|GetMoving))
  (bind _output_get_2 (Variables|Default|SetYPositionBeforeMove (.Y (Math|Vector|BreakVector (Transformation|GetActorLocation)))))
  (if (> _output_get _output_get_2)
    (Variables|Default|SetIsMovedRight true)
    (Variables|Default|SetIsMoveLeftInterrupted true)
    (Variables|Default|SetIsMoveRighInterrupted false)
    (bind _alpha (Timeline|Moving PlayFromStart)
      (:Update
        (Transformation|SetActorLocation (Math|Vector|MakeVector _x (Math|Float|Lerp (Variables|Default|GetYPositionBeforeMove) _output_get _alpha) _z) false false))
      (:Finished
        (Variables|Default|SetIsMovedLeft false)
        (Variables|Default|SetIsMovedRight false)))
    (else
      (Variables|Default|SetIsMovedLeft true)
      (Variables|Default|SetIsMoveRighInterrupted true)
      (Variables|Default|SetIsMoveLeftInterrupted false)
      (Timeline|Moving PlayFromStart))))

(event EventTick
  (params (DeltaSeconds :type Float%20%28single-precision%29))
  (bind _returnvalue (Transformation|GetActorLocation))
  (bind (_x _y _z) (Math|Vector|BreakVector _returnvalue))
  ;[1 0.01949 0] Посмотреть, как оставлять персонажа на месте с помощью физики
  (bind _output_get (Variables|Default|SetXShiftValueAccumulator (+ (Variables|Default|GetXShiftValueAccumulator) (Variables|Default|GetXShiftValue))))
  (Transformation|SetActorLocation (Math|Vector|MakeVector _output_get _y _z) false false)
  (if (< (.Z (Math|Vector|BreakVector (Variables|/Script/Engine.MovementComponent|GetVelocity (Variables|Character|GetCharacterMovement)))) 0.0)
    (Variables|Default|SetIsDashingDown true)
    (else
      (Variables|Default|SetIsDashingDown false))))

(event EventBeginPlay
  ;[1 1 1] Pre Init (Попытка инициализации массива позиций, относительно платформы). На случай, если BeginPlay персонажа вызовется раньше, таймер будет крутить инициализацию, пока не найдет платформу.
  (CallFunction|BindLevelLimitertoRoot))

(fn ConstructionScript)

(fn GetMesh
  (return (Variables|Character|GetMesh)))

(fn IncrementPlatformsPassedCount
  (bind _result (Math|Integer|IncrementInt (Variables|Default|GetPlatformsPassedCount))
    (:%20%20
      (Variables|Default|SetPlatformsPassedCount (Math|Integer|Clamp(Integer) _result 0 10)))))

(fn ImroveSpeed
  (bind _charactermovement (Variables|Character|GetCharacterMovement))
  (Variables|/Script/Engine.CharacterMovementComponent|SetMaxWalkSpeed _charactermovement (+ (Variables|/Script/Engine.CharacterMovementComponent|GetMaxWalkSpeed _charactermovement) 1e+02))
  (Variables|Default|SetPlatformsPassedCount 0))

(fn GetIsCharacterDead
  (return (Variables|Default|GetIsCharacterDead)))

(fn GetIsCharacterLanded
  (return (Variables|Default|GetIsCharacterLanded)))

(fn SetIsCharacterLanded
  (params (IsCharacterLanded :type Boolean))
  (Variables|Default|SetIsCharacterLanded IsCharacterLanded))

(fn SetPoints
  (params (PointsNumber :type Integer))
  (Variables|Default|SetPointsNumber (+ (Variables|Default|GetPointsNumber) PointsNumber)))

(fn KillCharacterWithoutPhysics
  (params (HitAnimation :type E_HitAnimation%20Enum :default "NewEnumerator0"))
  (Variables|Default|SetCurrentHitAnimation HitAnimation)
  (Transformation|AttachComponentToComponent (Variables|MyCharacter|GetCameraBoom) 0 "None" "KeepRelative" "KeepRelative" "KeepRelative" true)
  (Variables|Default|SetIsCharacterDead true))

(fn GetIsMovedLeft
  (return (Variables|Default|GetIsMovedLeft)))

(fn GetIsMovedRight
  (return (Variables|Default|GetIsMovedRight)))

(fn GetIsMoveLeftInterrupted
  (return (Variables|Default|GetIsMoveLeftInterrupted)))

(fn GetIsMoveRightInterrupted
  (return (Variables|Default|GetIsMoveRighInterrupted)))

(fn DashDown
  (if (== (.Z (Math|Vector|BreakVector (Transformation|GetVelocity))) 0.0)
    (Variables|Default|SetIsDashingDown false)
    (Variables|Default|SetIsRolling true)
    (Utilities|Time|ClearTimerbyFunctionName 0 "DashDown")
    (else
      (Variables|/Script/Engine.MovementComponent|SetVelocity (Variables|Character|GetCharacterMovement) (Math|Vector|MakeVector (.X (Math|Vector|BreakVector (Variables|/Script/Engine.MovementComponent|GetVelocity (Variables|Character|GetCharacterMovement)))) (.Y (Math|Vector|BreakVector (Variables|/Script/Engine.MovementComponent|GetVelocity (Variables|Character|GetCharacterMovement)))) (- (.Z (Math|Vector|BreakVector (Variables|/Script/Engine.MovementComponent|GetVelocity (Variables|Character|GetCharacterMovement)))) 35.0))))))

(fn GetIsDashingDown
  (return (Variables|Default|GetIsDashingDown)))

(fn KillCharacterwithPhysics
  (Collision|SetCollisionEnabled (Variables|Collision|GetCapsuleComponent) "NoCollision")
  (bind _skeletalmeshcomponent (CallFunction|GetMesh))
  (Physics|SetSimulatePhysics _skeletalmeshcomponent true)
  (Class|SkeletalMeshComponent|AddImpulsetoAllBodiesBelow _skeletalmeshcomponent "1350.000000, 0,870.000000" "None" true true)
  (Variables|Default|SetIsCharacterDead true))

(fn GetIsRolling
  (return (Variables|Default|GetIsRolling)))

(fn ResetStateAfterRoll
  (Variables|Default|SetIsRolling false)
  (Collision|SetCollisionEnabled (Variables|Collision|GetCapsuleComponent) "QueryAndPhysics"))

(fn RollUndertheFenceifRangeIsValid
  (params (Fence :type BP%20Fence%20Object%20Reference))
  (if (not (< (- (.X (Math|Vector|BreakVector (Transformation|GetActorLocation Fence))) (.X (Math|Vector|BreakVector (Transformation|GetActorLocation)))) 2.5e+02))
    (Collision|SetCollisionEnabled (Variables|Collision|GetCapsuleComponent) "NoCollision")))

(fn DoJump
  (if (not (Variables|Default|GetIsCharacterDead))
    (Variables|Default|SetIsCharacterLanded false)
    (Character|Jump)))

(fn StartDashDown
  (bind _returnvalue (Transformation|GetActorLocation))
  ;[1 1 1] Если мы не в прыжке, то кувырок, а если в прыжке - то рывок и кувырок
  (if (== (.Z (Math|Vector|BreakVector (Variables|/Script/Engine.MovementComponent|GetVelocity (Variables|Character|GetCharacterMovement)))) 0.0)
    (Variables|Default|SetIsRolling true)
    (bind _outhit (Collision|LineTraceByChannel _returnvalue (+ _returnvalue "400.000000, 0, 0") "TraceTypeQuery1" false 0 "None"))
    (bind _asbp_fence (Utilities|Casting|CastToBP_Fence (.HitActor (Collision|BreakHitResult _outhit))))
    (CallFunction|RollUndertheFenceifRangeIsValid _asbp_fence)
    (else
      (Variables|Default|SetIsDashingDown true)
      (Utilities|Time|SetTimerbyFunctionName 0 "DashDown" 0.001 true))))

(fn DoSuperJump
  (Variables|/Script/Engine.CharacterMovementComponent|SetJumpZVelocity (Variables|Character|GetCharacterMovement) 7e+02)
  (CallFunction|DoJump)
  (Variables|Default|SetXShiftValue 1e+01))

(fn CheckforRunningState
  (Utilities|FlowControl|Sequence
    (:then_0
      (if (Variables|Default|GetIsMovedLeft)
        (return false)))
    (:then_1
      (if (Variables|Default|GetIsMovedRight)
        (return false)))
    (:then_2
      (if (Variables|Default|GetIsDashingDown)
        (return false)))
    (:then_3
      (if (Variables|Default|GetIsRolling)
        (return false)))
    (:then_4
      (return true))))

(fn BindLevelLimitertoRoot
  ;[1 1 1] Во время супер прыжка придется тянуть оверлаппер за собой, потому как спавн платформ впереди должен оставаться с той же интенсивностью
  (bind _outactors (Actor|GetAllActorsOfClass "/Game/LookAroundGame/Blueprints/BP_LevelLimiter.BP_LevelLimiter_C"))
  (Transformation|AttachComponentToComponent (Utilities|Array|Get(acopy) _outactors) (Variables|Collision|GetCapsuleComponent) "None" "KeepRelative" "KeepRelative" "KeepRelative" true))

(fn StopMove
  (Variables|Default|SetIsMovedLeft false)
  (Variables|Default|SetIsMovedRight false)
  (Audio|Components|Audio|Stop (Variables|Default|GetMoving)))

(fn GetCurrentHitAnimation
  (return (Variables|Default|GetCurrentHitAnimation)))

(fn GetIsCharacterCurrentPositionMoreThanNew
  (return (> (.Y (Math|Vector|BreakVector (Transformation|GetActorLocation))) (Variables|Default|GetNewYPosition))))