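; Player controller for a three-lane runner-style game that turns move, dash and jump input into BP_Character actions.
; On BeginPlay it caches the character and polls on a looping timer until a BP_Platform exists, then stores that platform's lane Y positions.
; Left and right input step a bounded lane index, unless the character is dead, and pass the new Y to DoMove.
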(event EventBeginPlay
  (bind _asbp_character (Utilities|Casting|CastToBP_Character (Pawn|GetControlledPawn)))
  (Variables|Default|SetThirdPersonCharacter _asbp_character)
  (Utilities|Time|SetTimerbyFunctionName 0 "InitYPositions" 0.001 true))

(event Input|ActionEvents|InputActionMoveRight
  (params (Key :type Key%20Structure :default "None"))
  (:Pressed
    (if (and (not (Default|GetIsCharacterDead (Variables|Default|GetThirdPersonCharacter))) (< (Variables|Default|GetCurrentCharacterPositionIndex) 2))
      (bind _nextcharacteryposition (CallFunction|CalculateCharacterNewYPosition "NewEnumerator1"))
      (Default|DoMove (Variables|Default|GetThirdPersonCharacter) _nextcharacteryposition))))

(event Input|ActionEvents|InputActionMoveLeft
  (params (Key :type Key%20Structure :default "None"))
  (:Pressed
    (if (and (not (Default|GetIsCharacterDead (Variables|Default|GetThirdPersonCharacter))) (> (Variables|Default|GetCurrentCharacterPositionIndex) 0))
      (bind _nextcharacteryposition (CallFunction|CalculateCharacterNewYPosition "NewEnumerator0"))
      (Default|DoMove (Variables|Default|GetThirdPersonCharacter) _nextcharacteryposition))))

(event Input|ActionEvents|InputActionDash
  (params (Key :type Key%20Structure :default "None"))
  (:Pressed
    (Default|StartDashDown (Variables|Default|GetThirdPersonCharacter))))

(event Input|ActionEvents|InputActionJump
  (params (Key :type Key%20Structure :default "None"))
  (:Pressed
    (Default|DoJump (Variables|Default|GetThirdPersonCharacter))))

(fn ConstructionScript)

(fn CalculateCharacterNewYPosition
  (params (IndexCountType :type E_IndexCountType%20Enum :default "NewEnumerator0"))
  (switch Utilities|FlowControl|Switch|SwitchonE_IndexCountType IndexCountType
    (:NewEnumerator0
      (bind _result (Math|Integer|DecrementInt (Variables|Default|GetCurrentCharacterPositionIndex))
        (:%20%20
          (return (Utilities|Array|Get(acopy) (Variables|Default|GetYPositions) (Math|Integer|Clamp(Integer) _result 0 2))))))
    (:NewEnumerator1
      (bind _result_2 (Math|Integer|IncrementInt (Variables|Default|GetCurrentCharacterPositionIndex))
        (:%20%20
          (return (Utilities|Array|Get(acopy) (Variables|Default|GetYPositions) (Math|Integer|Clamp(Integer) _result_2 0 2))))))))

(fn InitYPositions
  (bind _outactors (Actor|GetAllActorsOfClass "/Game/LookAroundGame/Blueprints/Environment/BP_Platform.BP_Platform_C"))
  (Utilities|IsValid (Utilities|Array|Get(acopy) _outactors)
    (:Is%20Valid
      (bind _environmentscenecomponentsypositions (Default|GetEnvironmentSceneComponentsYPositions (Utilities|Array|Get(acopy) _outactors)))
      (Variables|Default|SetYPositions _environmentscenecomponentsypositions)
      ;[1 1 1] Останавливаем таймер, если платформу нашли
      (Utilities|Time|ClearTimerbyFunctionName 0 "InitYPositions"))))